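; Target actor that moves through the level and, when shot, pushes a RainbowCube in a color-coded direction.
; On BeginPlay it picks a random shape mesh and one of six color materials, which also sets its axis-aligned RainbowDirection.
; A hit from a FirstPersonProjectile calls MoveRainbowCube with that direction.
; Tick translates the actor along MoveDirection at MoveSpeed, scaled by delta time and without sweep.
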(event EventBeginPlay
  (bind _shape (Variables|Default|GetShape))
  (Variables|Default|SetColorIndex (Math|Random|RandomIntegerinRange 0 5))
  (Components|StaticMesh|SetStaticMesh _shape (Utilities|Select :Index (Math|Random|RandomIntegerinRange 0 4) :Option%200 "/Game/StarterContent/Shapes/Shape_Sphere.Shape_Sphere" :Option%201 "/Game/StarterContent/Shapes/Shape_Cylinder.Shape_Cylinder" :Option%202 "/Game/StarterContent/Shapes/Shape_Cube.Shape_Cube" :Option%203 "/Game/StarterContent/Shapes/Shape_Cone.Shape_Cone" :Option%204 "/Game/StarterContent/Shapes/Shape_Torus.Shape_Torus"))
  (Rendering|Material|SetMaterial _shape 0 (Utilities|Select :Index (Variables|Default|GetColorIndex) :Option%200 "/Game/Materials/Red.Red" :Option%201 "/Game/Materials/Yellow.Yellow" :Option%202 "/Game/Materials/White.White" :Option%203 "/Game/Materials/Green.Green" :Option%204 "/Game/Materials/Blue.Blue" :Option%205 "/Game/Materials/Orange.Orange"))
  (Variables|Default|SetRainbowDirection (Utilities|Select :Index (Variables|Default|GetColorIndex) :Option%200 (Math|Vector|VectorUp) :Option%201 (Class|KismetMathLibrary|VectorBackward) :Option%202 (Class|KismetMathLibrary|VectorForward) :Option%203 (Class|KismetMathLibrary|VectorLeft) :Option%204 (Class|KismetMathLibrary|VectorRight) :Option%205 (Math|Vector|VectorDown))))

(event EventTick
  (params (DeltaSeconds :type Float%20%28single-precision%29))
  (bind _defaultsceneroot (Variables|Default|GetDefaultSceneRoot))
  (bind _returnvalue (Transformation|GetWorldTransform _defaultsceneroot))
  ;[1 1 1] Move Every Frame
  (Transformation|SetActorTransform (Math|Transform|MakeTransform (+ (* (Variables|Default|GetMoveDirection) (* DeltaSeconds (Variables|Default|GetMoveSpeed))) (.location _returnvalue)) (.rotation _returnvalue) (.scale _returnvalue))))

(event Collision|EventHit
  (params (MyComp :type Primitive%20Component%20Object%20Reference) (Other :type Actor%20Object%20Reference) (OtherComp :type Primitive%20Component%20Object%20Reference) (bSelfMoved :type Boolean) (HitLocation :type Vector :default "0, 0, 0") (HitNormal :type Vector :default "0, 0, 0") (NormalImpulse :type Vector :default "0, 0, 0") (Hit :type Hit%20Result%20Structure%20%28by%20ref%29))
  (if (== (Utilities|GetClass Other) "/Game/FirstPersonBP/Blueprints/FirstPersonProjectile.FirstPersonProjectile_C")
    (Default|MoveRainbowCube (Variables|Default|GetRainbowCube) (Variables|Default|GetRainbowDirection))))

(fn ConstructionScript)