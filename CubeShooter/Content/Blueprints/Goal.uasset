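; Goal actor that the first-person character chases for points and extra time in a timed game.
; On BeginPlay and on each player overlap it teleports to a random point in a spawn box; overlaps also play an explosion sound.
; A Teleporting flag with a short Delay guards re-triggering, but non-player overlaps never clear it.
; Tick uses a one-second Delay as the countdown, creating a GameOver widget whenever time is depleted.
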(event EventBeginPlay
  (CallFunction|TeleportRandom))

(event Collision|EventActorBeginOverlap
  (params (OtherActor :type Actor%20Object%20Reference))
  (if (not (Variables|Default|GetTeleporting))
    (Variables|Default|SetTeleporting true)
    (if (== (Utilities|GetClass OtherActor) "/Game/FirstPersonBP/Blueprints/FirstPersonCharacter.FirstPersonCharacter_C")
      (CallFunction|TeleportRandom)
      (Variables|Default|SetPoints (+ (Variables|Default|GetPoints) 1))
      (Variables|Default|SetTimeRemaining (+ (Variables|Default|GetTimeRemaining) (Variables|Default|GetRewardTime)))
      (Utilities|FlowControl|Delay 0.2)
      (Variables|Default|SetTeleporting false)
      (Audio|PlaySoundatLocation "/Game/StarterContent/Audio/Explosion01.Explosion01" (.location (Transformation|GetActorTransform)) "0, 0, 0" 1.0 1.0 0.0 0 0 0))))

(event EventTick
  (params (DeltaSeconds :type Float%20%28single-precision%29))
  (Utilities|FlowControl|Delay 1.0)
  (bind _output_get (Variables|Default|SetTimeRemaining (- (Variables|Default|GetTimeRemaining) 1)))
  (if (<= _output_get 0) ; if no time remaing
    (Variables|Default|SetTimeRemaining 0)
    (bind _returnvalue (UserInterface|CreateWidget "/Game/Blueprints/GameOver.GameOver_C"))
    (UserInterface|Viewport|AddtoViewport _returnvalue 0)))

(fn ConstructionScript)

(fn TeleportRandom
  (bind _returnvalue (Transformation|GetActorTransform))
  (Transformation|SetActorTransform (Math|Transform|MakeTransform (Math|Random|RandomPointinBoundingBox (Variables|Default|GetSpawnCenter) (Variables|Default|GetSpawnExtents)) (.rotation _returnvalue) (.scale _returnvalue)) false true))