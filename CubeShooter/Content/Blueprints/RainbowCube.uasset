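; RainbowCube is an actor that slides along a given direction for a set distance at constant speed when MoveRainbowCube is called.
; The event ignores calls while moving, otherwise raises IsMoving and clears it after a delay of distance over speed.
; Tick feeds MoveOnTick, which offsets the actor from the mesh's world transform each frame without sweeping.
; An unconnected up-and-down test sequence never runs.
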(event Custom|MoveRainbowCube
  (params (Direction :type Vector))
  ;[1 1 1] On Move
  (if (not (Variables|Default|GetIsMoving))
    (Variables|Default|SetIsMoving true) ; Start moving every frame
    (Utilities|FlowControl|Delay (/ (Variables|Default|GetMoveDistance) (Variables|Default|GetMoveSpeed))) ; Wait until distance is covered
    (Variables|Default|SetIsMoving false) ; Finish Moving
  ))

(event EventBeginPlay)

(event Collision|EventActorBeginOverlap
  (params (OtherActor :type Actor%20Object%20Reference)))

(event EventTick
  (params (DeltaSeconds :type Float%20%28single-precision%29))
  (CallFunction|MoveonTick (stale Custom|MoveRainbowCube Direction) (Variables|Actor|GetRainbowCubeMesh) (Variables|Default|GetIsMoving) DeltaSeconds (Variables|Default|GetMoveSpeed)))

(fn ConstructionScript)

(fn MoveonTick
  (params (Direction :type Vector) (Target :type Scene%20Component%20Object%20Reference) (IsMoving :type Boolean) (DeltaSeconds :type Float%20%28single-precision%29) (MoveSpeed :type Float%20%28single-precision%29))
  (bind _returnvalue (Transformation|GetWorldTransform Target))
  ;[1 1 1] Move Every Frame
  (if IsMoving
    (Transformation|SetActorTransform (Math|Transform|MakeTransform (+ (* Direction (* DeltaSeconds MoveSpeed)) (.location _returnvalue)) (.rotation _returnvalue) (.scale _returnvalue)))))