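; SnitchTarget is a gold-colored bonus target that grants extra time when shot.
; On BeginPlay it applies a gold metal material to its shape mesh and calls its parent's BeginPlay, as Tick and construction do.
; When hit by a FirstPersonProjectile, it finds the first Goal actor in the level, adds RewardTime to that actor's TimeRemaining, and destroys itself.
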(event EventBeginPlay
  (|CallParentFunction)
  (Rendering|Material|SetMaterial (Variables|Default|GetShape) 0 "/Game/StarterContent/Materials/M_Metal_Gold.M_Metal_Gold"))

(event Collision|EventActorBeginOverlap
  (params (OtherActor :type Actor%20Object%20Reference)))

(event EventTick
  (params (DeltaSeconds :type Float%20%28single-precision%29))
  (|CallParentFunction DeltaSeconds))

(event Collision|EventHit
  (params (MyComp :type Primitive%20Component%20Object%20Reference) (Other :type Actor%20Object%20Reference) (OtherComp :type Primitive%20Component%20Object%20Reference) (bSelfMoved :type Boolean) (HitLocation :type Vector :default "0, 0, 0") (HitNormal :type Vector :default "0, 0, 0") (NormalImpulse :type Vector :default "0, 0, 0") (Hit :type Hit%20Result%20Structure%20%28by%20ref%29))
  (if (== (Utilities|GetClass Other) "/Game/FirstPersonBP/Blueprints/FirstPersonProjectile.FirstPersonProjectile_C")
    (bind _outactors (Actor|GetAllActorsOfClass "/Game/Blueprints/Goal.Goal_C"))
    (Variables|/Game/Blueprints/Goal.Goal_C|SetTimeRemaining (Utilities|Array|Get(acopy) _outactors) (+ (Variables|/Game/Blueprints/Goal.Goal_C|GetTimeRemaining (Utilities|Array|Get(acopy) _outactors)) (Variables|Default|GetRewardTime)))
    (Actor|DestroyActor)))

(fn ConstructionScript
  (|CallParentFunction))